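; BP_SwarmManager is an actor that spawns and keeps track of a swarm of boids.
; On BeginPlay it spawns a configurable number of BP_Boid actors at random positions within a min/max spawn range and stores each in the Swarm array.
; Tick loops over the Swarm array, but the loop body is empty, so the manager applies no flocking behavior.
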(event `self.ReceiveBeginPlay`
  (bind (_spawnrangemin_x _spawnrangemin_y _spawnrangemin_z) (`KismetMathLibrary.BreakVector` (`self.SpawnRangeMin`)))
  (bind (_spawnrangemax_x _spawnrangemax_y _spawnrangemax_z) (`KismetMathLibrary.BreakVector` (`self.SpawnRangeMax`)))
  ;[0.2008 1 0.1428] Spawning in number of boids to spawn at random locations
  (for _ (range (`self.NumberOfBoidsToSpawn`))
    (bind _returnvalue (`|SpawnActorFromClass` "/Game/Boids/Blueprints/BP_Boid.BP_Boid_C" (`KismetMathLibrary.Conv_VectorToTransform` (`KismetMathLibrary.MakeVector` (`KismetMathLibrary.RandomFloatInRange` _spawnrangemin_x _spawnrangemax_x) (`KismetMathLibrary.RandomFloatInRange` _spawnrangemin_y _spawnrangemax_y) (`KismetMathLibrary.RandomFloatInRange` _spawnrangemin_z _spawnrangemax_z))) "Undefined" "MultiplyWithRoot" null null))
    (`KismetArrayLibrary.Array_Add` (`self.Swarm`) _returnvalue)))

(event `self.ReceiveTick`
  (params (DeltaSeconds :type "Float (single-precision)"))
  (for _ (`self.Swarm`)
    _))

(fn `UserConstructionScript`)