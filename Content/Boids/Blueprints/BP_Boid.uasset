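; Boid actor that roams on its own using wander steering, with no flocking behavior in this Blueprint.
; At a short fixed interval, Wander picks a random point on a sphere projected ahead and Seek turns it into a clamped steering force.
; Each Tick, UpdateMovement adds accumulated acceleration to velocity, clamps it by MaxForce and applies it as a local offset without delta-time scaling.
; Debug drawing shows the wander sphere and target.
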(event `self.ReceiveTick`
  (params (DeltaSeconds :type "Float (single-precision)"))
  (bind (_forwardlocation _randomvectorfromforwardlocation) (`self.Wander` DeltaSeconds))
  ;[0 0.8199 1] Debug: For Forward Velocity Randomization (Attach to Event Tick)
  (`KismetSystemLibrary.DrawDebugLine` (`self.K2_GetActorLocation`) _forwardlocation (struct :`R` 0.095426 :`G` 1.0 :`A` 1.0) 0.0 1.0)
  (`KismetSystemLibrary.DrawDebugSphere` _forwardlocation (`self.WanderRadiusForRandomLocation`) 12 (struct :`G` 0.077228 :`B` 1.0 :`A` 1.0) 0.0 1.0)
  (`KismetSystemLibrary.DrawDebugPoint` _randomvectorfromforwardlocation 10.0 (struct :`R` 1.0 :`A` 1.0) 0.5)
  (`self.UpdateMovement`))

(fn `ApplyForce`
  (params (Force :type "Vector Structure"))
  ;[0.2008 1 0.1428] Add a given force to current accleration
  (set `self.Accleration` (+ (`self.Accleration`) Force)))

(fn `Seek`
  (params (Target :type "Vector Structure"))
  (bind _maxforce (`self.MaxForce`))
  (set `self.WanderDesiredDirection` (* (`KismetMathLibrary.Normal` (- Target (`self.K2_GetActorLocation`))) (`self.Speed`)))
  (bind _output_get (set `self.WanderSteering` (`KismetMathLibrary.ClampVectorSize` (- (`self.WanderDesiredDirection`) (`self.CurrentVelocity`)) (* _maxforce -1.0) _maxforce)))
  (`KismetSystemLibrary.PrintString` (`KismetStringLibrary.Conv_VectorToString` _output_get))
  (`self.ApplyForce` _output_get))

(fn `UpdateMovement`
  ;[1 1 1] Adding the accleration to the current velocity
  (bind _output_get (set `self.CurrentVelocity` (+ (`self.CurrentVelocity`) (`self.Accleration`))))
  ;[1 1 1] Limit the velocity to the max speed
  (bind _output_get_2 (set `self.CurrentVelocity` (`KismetMathLibrary.Vector_ClampSizeMax` _output_get (`self.MaxForce`))))
  ;[1 1 1] Change actor position
  (`self.K2_AddActorLocalOffset` _output_get_2 false true)
  ;[1 1 1] Reset acceleration
  (set `self.Accleration` (0.0 0.0 0.0)))

(fn `UserConstructionScript`)

(fn `Wander`
  (params (DeltaTime :type "Float (double-precision)"))
  (returns (ForwardLocation :type "Vector Structure") (RandomVectorFromForwardLocation :type "Vector Structure"))
  (bind _wandertarget (`self.WanderTarget`))
  (bind _returnvalue (+ (`self.K2_GetActorLocation`) (* (`self.GetActorForwardVector`) (`self.ForwardDistanceForRandomLocation`))))
  (set `self.WanderElapsedTime` (+ (`self.WanderElapsedTime`) DeltaTime))
  (if (>= (`self.WanderElapsedTime`) 0.2)
    (set `self.WanderElapsedTime` 0.0)
    (set `self.WanderTheta` (`KismetMathLibrary.RandomUnitVector`))
    (bind _output_get (set `self.WanderTarget` (+ (* (`self.WanderTheta`) (`self.WanderRadiusForRandomLocation`)) _returnvalue)))
    (`self.Seek` _wandertarget)
    ;[0.2008 1 0.1428] Returning information for debugs
    (return _returnvalue _wandertarget)))